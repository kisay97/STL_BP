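; BP_MinimapCapturer is an actor for the minimap that holds an orthographic SceneCaptureComponent2D and exposes zoom controls for it.
; ZoomIn and ZoomOut change the capture's OrthoWidth by ZoomStep, clamping it to OrthoMin and OrthoMax respectively.
; The event graph and construction script are empty, so zooming happens only when these functions are called.
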(fn `UserConstructionScript`)

(fn `ZoomIn`
  (bind _returnvalue (- (`SceneCaptureComponent2D.OrthoWidth` (`self.SceneCaptureComponent2D`)) (`self.ZoomStep`)))
  (if (< _returnvalue (`self.OrthoMin`))
    (set `SceneCaptureComponent2D.OrthoWidth` (`self.OrthoMin`) (`self.SceneCaptureComponent2D`))
    (else
      (set `SceneCaptureComponent2D.OrthoWidth` _returnvalue (`self.SceneCaptureComponent2D`)))))

(fn `ZoomOut`
  (bind _returnvalue (+ (`SceneCaptureComponent2D.OrthoWidth` (`self.SceneCaptureComponent2D`)) (`self.ZoomStep`)))
  (if (> _returnvalue (`self.OrthoMax`))
    (set `SceneCaptureComponent2D.OrthoWidth` (`self.OrthoMax`) (`self.SceneCaptureComponent2D`))
    (else
      (set `SceneCaptureComponent2D.OrthoWidth` _returnvalue (`self.SceneCaptureComponent2D`)))))