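; Actor component that sets up minimap capture for the actor that owns it.
; On BeginPlay it spawns a BP_MinimapCapturer at the owner's location, attaches it with snap-to-target rules and stores the reference.
; A branch that would create the UMG_Minimap widget for player controller 0 is present but unconnected, so this component never creates the minimap UI.
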(event `self.ReceiveBeginPlay`
  (`|ExecutionSequence`
    (:`then_0`
      (`self.SpawnAndAttachMimimapCapturer`))))

(fn `SpawnAndAttachMimimapCapturer`
  (bind _returnvalue (`self.GetOwner`))
  (bind _returnvalue_2 (`|SpawnActorFromClass` "/Game/Minimap/BP_MinimapCapturer.BP_MinimapCapturer_C" (`KismetMathLibrary.MakeTransform` (`Actor.K2_GetActorLocation` _returnvalue)) "AlwaysSpawn" "OverrideRootScale" null null))
  (`Actor.K2_AttachToActor` _returnvalue_2 _returnvalue "None" "SnapToTarget" "SnapToTarget" "SnapToTarget" true)
  (set `self.BP_MinimapCapturer` _returnvalue_2))