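; BP_AFountain is a fountain actor that spins through a RotatingMovement component, with keyboard controls for testing.
; H toggles the component, J and K lower or raise the yaw speed, and P prints the current speed.
; Speed changes, including an initial bump on BeginPlay, go through one additive function that updates RotationRate.
; Tick calls an empty function whose manual Castle rotation is disconnected; on-screen prints report activation changes.
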(event `self.ReceiveBeginPlay`
  (`KismetSystemLibrary.PrintString` "Hello World!" true false (struct :`R` 1.0 :`A` 1.0) 10.0)
  (`KismetSystemLibrary.PrintString` (`KismetStringLibrary.Conv_IntToString` 5) true false (struct :`R` 1.0 :`A` 1.0) 10.0)
  (`self.도는 속도 지정` 10.0))

(event `self.ReceiveTick`
  (params (DeltaSeconds :type "Float (single-precision)"))
  (`self.돌아라 설월화` DeltaSeconds))

(event `self.RotatingMovement.OnComponentActivated`
  (params (Component :type "ActorComponent Object Reference") (bReset :type Boolean))
  (`KismetSystemLibrary.PrintString` "돈다~ 돌아~" true true (struct :`R` 1.0 :`A` 1.0)))

(event `self.RotatingMovement.OnComponentDeactivated`
  (params (Component :type "ActorComponent Object Reference"))
  (`KismetSystemLibrary.PrintString` "멈춰!" true true (struct :`R` 1.0 :`A` 1.0)))

(event `Key|H`
  (params (Key :type "Key Structure"))
  (bind _rotatingmovement (`self.RotatingMovement`))
  (:`Pressed`
    (if (`ActorComponent.IsActive` _rotatingmovement)
      (`ActorComponent.Deactivate` _rotatingmovement)
      (else
        (`ActorComponent.Activate` _rotatingmovement false)))))

(event `Key|J`
  (params (Key :type "Key Structure"))
  (:`Pressed`
    (`self.느려져라 얍`)))

(event `Key|K`
  (params (Key :type "Key Structure"))
  (:`Pressed`
    (`self.빨라져라 얍`)))

(event `Key|P`
  (params (Key :type "Key Structure"))
  (:`Pressed`
    (`KismetSystemLibrary.PrintString` (`KismetStringLibrary.Concat_StrStr` "현재속도: " (`KismetStringLibrary.Conv_DoubleToString` (`self.도는속도`))) true false (struct :`R` 1.0 :`A` 1.0) 5.0)))

(fn `UserConstructionScript`)

(fn `느려져라 얍`
  (`self.도는 속도 지정` -10.0))

(fn `도는 속도 지정`
  (params (`변할 속도` :type "Float (double-precision)" :default 10.0))
  (bind _output_get (set `self.도는속도` (+ (`self.도는속도`) `변할 속도`)))
  (set `RotatingMovementComponent.RotationRate` (`KismetMathLibrary.MakeRotator` 0.0 0.0 _output_get) (`self.RotatingMovement`)))

(fn `돌아라 설월화`
  (params (DeltaTime :type "Float (double-precision)")))

(fn `빨라져라 얍`
  (`self.도는 속도 지정` 10.0))