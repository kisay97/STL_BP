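; BP_ATorch is a torch actor whose PSFire particle effect can be lit and put out.
; Actor overlap events track whether the player's controlled pawn is in range through the Overlap flag.
; Interaction calls OnTorch when the fire is already active or Overlap is set, so it never extinguishes.
; OnTorch and OffTorch switch the particles and also overwrite Overlap; nothing in this Blueprint calls OffTorch.
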(event `self.ReceiveActorBeginOverlap`
  (params (OtherActor :type "Actor Object Reference"))
  (set `self.bOverlap` (== OtherActor (`Controller.K2_GetPawn` (`GameplayStatics.GetPlayerController` 0)))))

(event `self.ReceiveActorEndOverlap`
  (params (OtherActor :type "Actor Object Reference"))
  (if (== OtherActor (`Controller.K2_GetPawn` (`GameplayStatics.GetPlayerController` 0)))
    (set `self.bOverlap` false)))

(event `/Game/Blueprints/Interface/BPI_Interact.Interaction`
  (if (or (`ActorComponent.IsActive` (`self.PS_Fire`)) (`self.bOverlap`))
    (`self.OnTorch`)))

(event `OffTorch`
  (set `self.bOverlap` false)
  (`ActorComponent.SetActive` (`self.PS_Fire`) false false))

(event `OnTorch`
  (set `self.bOverlap` true)
  (`ActorComponent.SetActive` (`self.PS_Fire`) true false))

(fn `UserConstructionScript`)