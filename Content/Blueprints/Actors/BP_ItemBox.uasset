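; BP_ItemBox is a pickup actor that gives an overlapping BP_Character a randomized weapon.
; Its construction script picks the box's static mesh at random from ItemMeshes.
; On overlap, it asks the character whether it can get a weapon, then spawns a Weapon, assigns a random skeletal mesh from WeaponMeshes and adds it to a slot.
; Otherwise it only prints a debug message, and the box itself stays in place after pickup.
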(event `self.StaticMesh.OnComponentBeginOverlap`
  (params (OverlappedComponent :type "PrimitiveComponent Object Reference") (OtherActor :type "Actor Object Reference") (OtherComp :type "PrimitiveComponent Object Reference") (OtherBodyIndex :type Integer) (bFromSweep :type Boolean) (SweepResult :type "HitResult Structure (by ref)"))
  (bind _asbp_character (cast `/Game/Blueprints/Actors/BP_Character` OtherActor))
  (`KismetSystemLibrary.PrintString` "ItemBoxOverlap")
  (bind _bcangetweapon (`/Game/Blueprints/Actors/BP_Character.CanGetWeapon` _asbp_character))
  (if _bcangetweapon
    (bind _returnvalue (`|SpawnActorFromClass` (`self.Weapon`) (`KismetMathLibrary.MakeTransform` (0.0 0.0 0.0)) "AlwaysSpawn" "OverrideRootScale" _asbp_character null))
    (`SkinnedMeshComponent.SetSkinnedAssetAndUpdate` (`/Game/Blueprints/Actors/BP_Weapon.SkeltalMesh` _returnvalue) (`KismetArrayLibrary.Array_Random` (`self.WeaponMeshes`)) true)
    (`/Game/Blueprints/Actors/BP_Character.Add Weapon to Slot` _asbp_character _returnvalue)
    (else
      (`KismetSystemLibrary.PrintString` "꽊참"))))

(fn `UserConstructionScript`
  (`StaticMeshComponent.SetStaticMesh` (`self.StaticMesh`) (`KismetArrayLibrary.Array_Random` (`self.ItemMeshes`))))