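; BP_Spawner is an actor that fills a box volume with instances of a configurable class, apparently bears, up to a maximum count.
; On BeginPlay it spawns the full count at random points in the box, records each in a list, and sets itself as each one's ParentSpawner.
; RemoveDeadBear drops an actor from that list, and CheckList spawns one replacement when below the cap, alongside a five-second looping timer.
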(event `self.ReceiveBeginPlay`
  (for _ (range 1 (+ (`self.MaxSpawned`) 1))
    (`self.SpawnActorByClass`))
  (`KismetSystemLibrary.K2_SetTimerDelegate` (`|CreateDelegate` :!event `CheckList`) 5.0 true))

(event `RemoveDeadBear`
  (params (DeleteBear :type "/Game/Blueprints/Actors/Bear/BP_Bear Object Reference"))
  (`KismetArrayLibrary.Array_RemoveItem` (`self.SpawnedActorList`) DeleteBear)
  (`KismetSystemLibrary.PrintString` "RemoveDeadBear"))

(event `CheckList`
  (if (< (`KismetArrayLibrary.Array_Length` (`self.SpawnedActorList`)) (`self.MaxSpawned`))
    (`self.SpawnActorByClass`)))

(fn `SpawnActorByClass`
  (bind (_origin _boxextent) (`KismetSystemLibrary.GetComponentBounds` (`self.Box`)))
  (bind _returnvalue (`|SpawnActorFromClass` (`self.Spawn_Class`) (`KismetMathLibrary.MakeTransform` (`KismetMathLibrary.RandomPointInBoundingBox` _origin _boxextent)) "AdjustIfPossibleButAlwaysSpawn" "OverrideRootScale" null "NewEnumerator0" null))
  (set `/Game/Blueprints/Actors/Bear/BP_Bear.ParentSpawner` self _returnvalue)
  (`KismetArrayLibrary.Array_Add` (`self.SpawnedActorList`) _returnvalue)
  (return))

(fn `UserConstructionScript`)