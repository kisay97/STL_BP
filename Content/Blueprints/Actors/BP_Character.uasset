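; Player character with camera-relative movement, mouse-wheel zoom, overlap-based BPI_Interact interaction, two swappable socketed weapon slots and a HUD.
; Attacks chain montage combos through AnimInstance events, while Tick sphere-traces between weapon trail sockets during IsAttackCheck, ignoring already-hit actors.
; Level stats come from BP_GameInstance and drive damage, EXP level-ups and death with delayed PlayerStart respawn.
; BeginPlay restores save data, rebuilding weapon meshes through Asset Registry lookups.
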(event `InputAction|Jump`
  (params (Key :type "Key Structure"))
  (:`Pressed`
    (`self.Jump`))
  (:`Released`
    (`self.StopJumping`) ; 살짝 점프, 긴 점프 같은 것을 처리할 수 있음.\n기본적으로 그런 기능을 넣지 않더라도 Stop Jumping은 Jump 입력 액션 Released에 넣어준다고 함.
  ))

(event `self.OnJumped`)

(event `InputAxisKey|MouseWheelAxis`
  (params (AxisValue :type "Float (single-precision)"))
  (bind _springarm (`self.SpringArm`))
  (set `SpringArmComponent.TargetArmLength` (+ (* AxisValue -10.0) (`SpringArmComponent.TargetArmLength` _springarm)) _springarm))

(event `InputAxis|MoveForward / MoveBackward`
  (params (AxisValue :type "Float (single-precision)"))
  (bind (_returnvalue_roll _returnvalue_pitch _returnvalue_yaw) (`KismetMathLibrary.BreakRotator` (`self.GetControlRotation`)))
  (`self.AddMovementInput` (`KismetMathLibrary.GetForwardVector` (`KismetMathLibrary.MakeRotator` 0.0 0.0 _returnvalue_yaw)) AxisValue) ; 속도는 캐릭터가 들고있다.(가속도, 최대속도 등)\n조작계에 따른 내 캐릭터의 정방을 World Direction으로 줘야한다.
)

(event `InputAxis|MoveRight / MoveLeft`
  (params (AxisValue :type "Float (single-precision)"))
  (bind (_returnvalue_roll _returnvalue_pitch _returnvalue_yaw) (`KismetMathLibrary.BreakRotator` (`self.GetControlRotation`)))
  (`self.AddMovementInput` (`KismetMathLibrary.GetRightVector` (`KismetMathLibrary.MakeRotator` 0.0 0.0 _returnvalue_yaw)) AxisValue) ; 속도는 캐릭터가 들고있다.(가속도, 최대속도 등)
)

(event `InputAction|Interact`
  (params (Key :type "Key Structure"))
  ;[1 1 1] 인터렉션. Interact Target이 유효할 경우 메시지 전달.
  (:`Pressed`
    (bind _interacttarget (`self.InteractTarget`)
      (:`then`
        (message `/Game/Blueprints/Interface/BPI_Interact.Interaction` _interacttarget))
      (:`else`))))

(event `InputAxis|TurnRight / Left`
  (params (AxisValue :type "Float (single-precision)"))
  (`self.AddControllerYawInput` AxisValue))

(event `self.InteractCollision.OnComponentBeginOverlap`
  (params (OverlappedComponent :type "PrimitiveComponent Object Reference") (OtherActor :type "Actor Object Reference") (OtherComp :type "PrimitiveComponent Object Reference") (OtherBodyIndex :type Integer) (bFromSweep :type Boolean) (SweepResult :type "HitResult Structure (by ref)"))
  ;[1 1 1] BPI있는 액터인 경우 레퍼런스 등록
  (if (`KismetSystemLibrary.DoesImplementInterface` OtherActor "/Game/Blueprints/Interface/BPI_Interact.BPI_Interact_C")
    (set `self.InteractTarget` OtherActor)))

(event `InputAxis|LookUp / Down`
  (params (AxisValue :type "Float (single-precision)"))
  (`self.AddControllerPitchInput` (/ AxisValue 3.0)))

(event `self.InteractCollision.OnComponentEndOverlap`
  (params (OverlappedComponent :type "PrimitiveComponent Object Reference") (OtherActor :type "Actor Object Reference") (OtherComp :type "PrimitiveComponent Object Reference") (OtherBodyIndex :type Integer))
  ;[1 1 1] 감지 해제 시 레퍼를 날려준다.
  (if (== OtherActor (`self.InteractTarget`))
    (set `self.InteractTarget` null)))

(event `InputAction|Attack`
  (params (Key :type "Key Structure"))
  (:`Pressed`
    (`/Engine/EditorBlueprintResources/StandardMacros.IsValid` (`self.CurrentWeapon`)
      (:`Is Valid`
        (`self.Attack`)))))

(event `InputAction|SwapWeapon1`
  (params (Key :type "Key Structure"))
  (:`Pressed`
    (`self.Swap Weapon1`)))

(event `InputAction|SwapWeapon2`
  (params (Key :type "Key Structure"))
  (:`Pressed`
    (`self.Swap Weapon2`)))

(event `self.ReceiveBeginPlay`
  (`|ExecutionSequence`
    (:`then_0`
      (`self.LoadCharacterData`))
    (:`then_1`
      (`self.DisableInput` (`GameplayStatics.GetPlayerController` 0))
      (bind _asabp_character (cast `/Game/Animations/ABP_Character` (`SkeletalMeshComponent.GetAnimInstance` (`self.Mesh`))))
      (bind _output_get (set `self.AnimInstance` _asabp_character))
      (add `/Game/Animations/ABP_Character.OnNextAttackCheck` _output_get (delegate `OnNextAttackCheck`))
      (add `/Game/Animations/ABP_Character.OnAttackMontageEnded` (`self.AnimInstance`) (delegate `OnAttackMontageEnded`))
      (bind _returnvalue (`|CreateWidget` "/Game/UI/UMG_PlayerHUD.UMG_PlayerHUD_C" (`GameplayStatics.GetPlayerController` 0)))
      (`UserWidget.AddToViewport` _returnvalue 0)
      (`KismetSystemLibrary.Delay` 2.5)
      (`self.EnableInput` (`GameplayStatics.GetPlayerController` 0)))))

(event `OnNextAttackCheck`
  (if (`self.bIsComboInputOn`)
    (`self.AttackStartCombo`)
    (`/Game/Animations/ABP_Character.JumpToAttackMontageSection` (`self.AnimInstance`) (`self.CurrentCombo`))
    (else
      (`AnimInstance.Montage_Stop` (`self.AnimInstance`) 0.3 null) ; Montage 안넣으면 기본으로 지금 재생중이던 몽타주를 스톱함
    )))

(event `OnAttackMontageEnded`
  (`self.AttackEndCombo`))

(event `OnAttackCheck`
  (`self.AttackCheck`))

(event `self.ReceiveTick`
  (params (DeltaSeconds :type "Float (single-precision)"))
  (`self.AttackCheck`))

(event `self.ReceiveAnyDamage`
  (params (Damage :type "Float (single-precision)") (DamageType :type "DamageType Object Reference") (InstigatedBy :type "Controller Object Reference") (DamageCauser :type "Actor Object Reference"))
  (`KismetSystemLibrary.PrintString` (`KismetStringLibrary.Concat_StrStr` "Damage: " (`KismetStringLibrary.Conv_DoubleToString` Damage) ", Damage Causer: " (`KismetSystemLibrary.GetDisplayName` DamageCauser)) true true (struct :`R` 1.0 :`A` 1.0) 5.0)
  (`self.SetDamagedHP` Damage)
  (if (`self.bIsDead`)
    (`PrimitiveComponent.SetCollisionEnabled` (`self.CapsuleComponent`) "NoCollision") ; 죽은 캐릭터의 콜리전을 끄는 방법도 있음.\n이게 더 일반적으로 사용된다고 함.
    (`KismetSystemLibrary.Delay` 5.0)
    (`self.Respon`)
    (`PrimitiveComponent.SetCollisionEnabled` (`self.CapsuleComponent`) "QueryAndPhysics")))

(event `self.ReceivePointDamage`
  (params (Damage :type "Float (single-precision)") (DamageType :type "DamageType Object Reference") (HitLocation :type "Vector Structure") (HitNormal :type "Vector Structure") (HitComponent :type "PrimitiveComponent Object Reference") (BoneName :type Name) (ShotFromDirection :type "Vector Structure") (InstigatedBy :type "Controller Object Reference") (DamageCauser :type "Actor Object Reference") (HitInfo :type "HitResult Structure (by ref)")))

(event `self.ReceiveRadialDamage`
  (params (DamageReceived :type "Float (single-precision)") (DamageType :type "DamageType Object Reference") (Origin :type "Vector Structure") (HitInfo :type "HitResult Structure (by ref)") (InstigatedBy :type "Controller Object Reference") (DamageCauser :type "Actor Object Reference")))

(fn `Add Weapon to Slot`
  (params (NewWeapon :type "/Game/Blueprints/Actors/BP_Weapon Object Reference"))
  (if (not (`KismetSystemLibrary.IsValid` (`self.WeaponSlot1`)))
    (bind _output_get (set `self.WeaponSlot1` NewWeapon))
    (`self.K2_AttachToComponent` _output_get (`self.Mesh`) "WeaponSlot1" "SnapToTarget" "SnapToTarget" "SnapToTarget" true)
    (elif (not (`KismetSystemLibrary.IsValid` (`self.WeaponSlot2`)))
      (bind _output_get_2 (set `self.WeaponSlot2` NewWeapon))
      (`self.K2_AttachToComponent` _output_get_2 (`self.Mesh`) "WeaponSlot2" "SnapToTarget" "SnapToTarget" "SnapToTarget" true))))

(fn `Attack`
  (set `CharacterMovementComponent.MaxWalkSpeed` 50.0 (`self.CharacterMovement`))
  (if (`self.bIsAttaking`)
    ;[1 1 1] 콤보 입력 감지
    (set `self.bIsComboInputOn` true)
    (return)
    (elif (`NavMovementComponent.IsFalling` (`self.CharacterMovement`))
      (`/Game/Animations/ABP_Character.PlayAttackMontage` (`self.AnimInstance`))
      (set `self.CurrentCombo` (`self.MaxCombo`))
      (`/Game/Animations/ABP_Character.JumpToAttackMontageSection` (`self.AnimInstance`) (`self.MaxCombo`))
      (set `self.bCanNextCombo` false)
      (set `self.bIsComboInputOn` false)
      (set `self.bIsAttaking` true)
      (else
        (`self.AttackStartCombo`)
        (`/Game/Animations/ABP_Character.PlayAttackMontage` (`self.AnimInstance`))
        (set `self.bIsAttaking` true)))))

(fn `AttackCheck`
  (locals (StartLoc :type "Vector Structure") (EndLoc :type "Vector Structure"))
  (bind _mesh (`self.Mesh`))
  (bind (_currentcharacterdata_level _currentcharacterdata_maxhp _currentcharacterdata_attack) (break `/Game/Blueprints/F_CharacterData` (`self.CurrentCharacterData`)))
  (if (`self.bIsAttackCheck`)
    (bind _outhit (`KismetSystemLibrary.SphereTraceSingle` (`SceneComponent.GetSocketLocation` _mesh "Trail_Start") (`SceneComponent.GetSocketLocation` _mesh "Trail_End") 15.0 "TraceTypeQuery1" false (`self.HittedActor`) "ForDuration" true (struct :`R` 1.0 :`A` 1.0) (struct :`G` 1.0 :`A` 1.0) 2.0))
    (`KismetArrayLibrary.Array_AddUnique` (`self.HittedActor`) (`.HitActor` (`GameplayStatics.BreakHitResult` _outhit))) ; trace에 ActorToIgnore때문에\nADD로 해도 무방함
    (`GameplayStatics.ApplyDamage` (`.HitActor` (`GameplayStatics.BreakHitResult` _outhit)) _currentcharacterdata_attack (`self.GetController`) self)
    (else
      (return))))

(fn `AttackEndCombo`
  (set `self.bIsAttaking` false)
  (set `self.CurrentCombo` 0)
  (set `self.bCanNextCombo` false)
  (set `self.bIsComboInputOn` false)
  (set `CharacterMovementComponent.MaxWalkSpeed` 600.0 (`self.CharacterMovement`)))

(fn `AttackStartCombo`
  (set `self.bCanNextCombo` true)
  (set `self.bIsComboInputOn` false)
  (set `self.CurrentCombo` (`KismetMathLibrary.Clamp` (+ (`self.CurrentCombo`) 1) 1 (`self.MaxCombo`))))

(fn `CanGetWeapon`
  (returns (bCanGetWeapon :type Boolean))
  (return (not (and (`KismetSystemLibrary.IsValid` (`self.WeaponSlot1`)) (`KismetSystemLibrary.IsValid` (`self.WeaponSlot2`))))))

(fn `GetExp`
  (params (NewExp :type "Float (double-precision)"))
  (bind (_level _maxhp _attack _nextexp) (break `/Game/Blueprints/F_CharacterData` (`self.CurrentCharacterData`)))
  (bind _output_get (set `self.CurrentExp` (+ NewExp (`self.CurrentExp`))))
  (if (>= _output_get _nextexp)
    (`self.LevelUp` (- _output_get _nextexp))))

(fn `GetExpRatio`
  (returns (expRatio :type "Float (double-precision)"))
  (bind (_currentcharacterdata_level _currentcharacterdata_maxhp _currentcharacterdata_attack _currentcharacterdata_nextexp) (break `/Game/Blueprints/F_CharacterData` (`self.CurrentCharacterData`)))
  (return (/ (`self.CurrentExp`) _currentcharacterdata_nextexp)))

(fn `LevelUp`
  (params (remainExp :type "Float (double-precision)"))
  (`|ExecutionSequence`
    (:`then_0`
      (`KismetSystemLibrary.PrintString` "레벨업 이펙트 무언가"))
    (:`then_1`
      (bind _asbp_game_instance (cast `/Game/Blueprints/Actors/Bear/BP_GameInstance` (`GameplayStatics.GetGameInstance`)))
      ;[1 1 1] 레벨업 캐릭터의 데이터 신규 세팅
      (bind _characterdata (`/Game/Blueprints/Actors/Bear/BP_GameInstance.GetCharacterData` _asbp_game_instance (+ (`.Level_6_A1B1A0DB45A1143D48A07B92C6EA64AB` (break `/Game/Blueprints/F_CharacterData` (`self.CurrentCharacterData`))) 1)))
      (bind _output_get (set `self.CurrentCharacterData` _characterdata))
      (set `self.CurrentHP` (`.MaxHP_7_8FF068034D1DE5F5388B87AD55D1D83E` (break `/Game/Blueprints/F_CharacterData` _output_get))))
    (:`then_2`
      (set `self.CurrentExp` remainExp))))

(fn `LoadCharacterData`
  (locals (gameinst :type "/Game/Blueprints/Actors/Bear/BP_GameInstance Object Reference") (savedWeapon1 :type "/Game/Blueprints/Actors/BP_Weapon Object Reference") (savedWeapon2 :type "/Game/Blueprints/Actors/BP_Weapon Object Reference"))
  (bind (_pathpart _filenamepart) (`BlueprintPathsLibrary.Split` (`/Game/Blueprints/BP_Savegame.Weapon2Mesh` (`/Game/Blueprints/Actors/Bear/BP_GameInstance.LoadData` (`local.gameinst`)))))
  (bind (_pathpart_2 _filenamepart_2) (`BlueprintPathsLibrary.Split` (`/Game/Blueprints/BP_Savegame.Weapon1Mesh` (`/Game/Blueprints/Actors/Bear/BP_GameInstance.LoadData` (`local.gameinst`)))))
  (bind _asbp_game_instance (cast `/Game/Blueprints/Actors/Bear/BP_GameInstance` (`GameplayStatics.GetGameInstance`)))
  (set `local.gameinst` _asbp_game_instance)
  (`/Engine/EditorBlueprintResources/StandardMacros.IsValid` (`/Game/Blueprints/Actors/Bear/BP_GameInstance.LoadData` (`local.gameinst`))
    (:`Is Valid`
      (`|ExecutionSequence`
        (:`then_0`
          (`|ExecutionSequence`
            (:`then_0`
              (bind _characterdata (`/Game/Blueprints/Actors/Bear/BP_GameInstance.GetCharacterData` (`local.gameinst`) (`/Game/Blueprints/BP_Savegame.CharacterLevel` (`/Game/Blueprints/Actors/Bear/BP_GameInstance.LoadData` (`local.gameinst`)))))
              (set `self.CurrentCharacterData` _characterdata))
            (:`then_1`
              (set `self.CurrentHP` (`/Game/Blueprints/BP_Savegame.CurrentHP` (`/Game/Blueprints/Actors/Bear/BP_GameInstance.LoadData` (`local.gameinst`)))))
            (:`then_2`
              (set `self.CurrentExp` (`/Game/Blueprints/BP_Savegame.CurrentExp` (`/Game/Blueprints/Actors/Bear/BP_GameInstance.LoadData` (`local.gameinst`)))))
            (:`then_3`
              (if (not (`KismetStringLibrary.IsEmpty` (`/Game/Blueprints/BP_Savegame.Weapon1Mesh` (`/Game/Blueprints/Actors/Bear/BP_GameInstance.LoadData` (`local.gameinst`)))))
                (bind _returnvalue (`|SpawnActorFromClass` "/Game/Blueprints/Actors/BP_Weapon.BP_Weapon_C" (`KismetMathLibrary.MakeTransform` (0.0 0.0 0.0)) "AlwaysSpawn" "OverrideRootScale" self null))
                (set `local.savedWeapon1` _returnvalue)
                (bind (_outassetdata _returnvalue_2) (`AssetRegistry.GetAssetsByPath` (`AssetRegistryHelpers.GetAssetRegistry`) (`KismetStringLibrary.Conv_StringToName` _pathpart_2) false true))
                (if _returnvalue_2
                  (for _array_element _outassetdata
                    (if (and (`KismetStringLibrary.Contains` (`AssetRegistryHelpers.GetExportTextName` _array_element) _filenamepart_2) (== (`AssetRegistryHelpers.GetClass` _array_element) "/Script/Engine.SkeletalMesh"))
                      (bind `_as스켈레탈_메시` (cast `SkeletalMesh` (`AssetRegistryHelpers.GetAsset` _array_element))
                        (:`then`
                          (`SkinnedMeshComponent.SetSkinnedAssetAndUpdate` (`/Game/Blueprints/Actors/BP_Weapon.SkeltalMesh` (`local.savedWeapon1`)) `_as스켈레탈_메시` true)
                          (`self.Add Weapon to Slot` (`local.savedWeapon1`))
                          (break))
                        (:`CastFailed`
                          (`KismetSystemLibrary.PrintString` "무기 1 스켈레탈 메시 로드 실패" true true (struct :`R` 1.0 :`A` 1.0) 20.0))))))))
            (:`then_4`
              (if (not (`KismetStringLibrary.IsEmpty` (`/Game/Blueprints/BP_Savegame.Weapon2Mesh` (`/Game/Blueprints/Actors/Bear/BP_GameInstance.LoadData` (`local.gameinst`)))))
                (bind _returnvalue_3 (`|SpawnActorFromClass` "/Game/Blueprints/Actors/BP_Weapon.BP_Weapon_C" (`KismetMathLibrary.MakeTransform` (0.0 0.0 0.0)) "AlwaysSpawn" "OverrideRootScale" self null))
                (set `local.savedWeapon2` _returnvalue_3)
                (bind (_outassetdata_2 _returnvalue_4) (`AssetRegistry.GetAssetsByPath` (`AssetRegistryHelpers.GetAssetRegistry`) (`KismetStringLibrary.Conv_StringToName` _pathpart) false true))
                (if _returnvalue_4
                  (for _array_element_2 _outassetdata_2
                    (if (and (`KismetStringLibrary.Contains` (`AssetRegistryHelpers.GetExportTextName` _array_element_2) _filenamepart) (== (`AssetRegistryHelpers.GetClass` _array_element_2) "/Script/Engine.SkeletalMesh"))
                      (bind `_as스켈레탈_메시_2` (cast `SkeletalMesh` (`AssetRegistryHelpers.GetAsset` _array_element_2))
                        (:`then`
                          (`SkinnedMeshComponent.SetSkinnedAssetAndUpdate` (`/Game/Blueprints/Actors/BP_Weapon.SkeltalMesh` (`local.savedWeapon2`)) `_as스켈레탈_메시_2` true)
                          (`self.Add Weapon to Slot` (`local.savedWeapon2`))
                          (break))
                        (:`CastFailed`
                          (`KismetSystemLibrary.PrintString` "무기 2 스켈레탈 메시 로드 실패" true true (struct :`R` 1.0 :`A` 1.0) 20.0))))))))
            (:`then_5`
              (switch `int` (`/Game/Blueprints/BP_Savegame.CurrentWeaponIdx` (`/Game/Blueprints/Actors/Bear/BP_GameInstance.LoadData` (`local.gameinst`)))
                (:`1`
                  (`self.Swap Weapon1`))
                (:`2`
                  (`self.Swap Weapon2`))))
            (:`then_6`
              (`self.K2_SetActorLocation` (`/Game/Blueprints/BP_Savegame.Location` (`/Game/Blueprints/Actors/Bear/BP_GameInstance.LoadData` (`local.gameinst`)))))))
        (:`then_1`
          (set `/Game/Blueprints/Actors/Bear/BP_GameInstance.LoadData` null (`local.gameinst`)))))))

(fn `MyBoxTraceByChannel`
  (bind _returnvalue (+ (* (`self.GetActorForwardVector`) (`CapsuleComponent.CapsuleRadius` (`self.CapsuleComponent`))) (`self.K2_GetActorLocation`)))
  (`KismetSystemLibrary.BoxTraceSingle` :`Start` _returnvalue :`End` (+ _returnvalue (* (`self.GetActorForwardVector`) (`self.AttackRange`))) :`HalfSize` (* (`KismetMathLibrary.Vector_One`) 10.0) :`Orientation` (`KismetMathLibrary.MakeRotFromX` (`self.GetActorForwardVector`)) :`TraceChannel` "TraceTypeQuery3" :`DrawDebugType` "ForDuration" :`DrawTime` 20.0) ; Half Size: 박스 한 면의 가로 세로의 절반\nOrientation: 박스가 회전된 상태
)

(fn `MyCapsuleTraceByChannel`
  (bind _returnvalue (+ (* (`self.GetActorForwardVector`) (`CapsuleComponent.CapsuleRadius` (`self.CapsuleComponent`))) (`self.K2_GetActorLocation`)))
  (`KismetSystemLibrary.CapsuleTraceSingle` :`Start` _returnvalue :`End` (+ _returnvalue (* (`self.GetActorForwardVector`) (`self.AttackRange`))) :`Radius` 10.0 :`HalfHeight` 20.0 :`TraceChannel` "TraceTypeQuery3" :`DrawDebugType` "ForDuration" :`DrawTime` 20.0))

(fn `MySphereTraceByChannel`
  (bind _returnvalue (+ (* (`self.GetActorForwardVector`) (`CapsuleComponent.CapsuleRadius` (`self.CapsuleComponent`))) (`self.K2_GetActorLocation`)))
  (`KismetSystemLibrary.SphereTraceSingle` :`Start` _returnvalue :`End` (+ _returnvalue (* (`self.GetActorForwardVector`) (`self.AttackRange`))) :`Radius` 10.0 :`TraceChannel` "TraceTypeQuery3" :`DrawDebugType` "ForDuration" :`DrawTime` 20.0))

(fn `Respon`
  (bind (_currentcharacterdata_level _currentcharacterdata_maxhp) (break `/Game/Blueprints/F_CharacterData` (`self.CurrentCharacterData`)))
  (`|ExecutionSequence`
    (:`then_0`
      (bind _returnvalue (`GameplayStatics.GetActorOfClass` "/Script/Engine.PlayerStart"))
      (`self.K2_SetActorTransform` (`self.GetTransform` _returnvalue)))
    (:`then_1`
      (set `self.CurrentHP` _currentcharacterdata_maxhp)
      (set `self.bIsDead` false))
    (:`then_2`
      (`self.EnableInput` (`GameplayStatics.GetPlayerPawn` 0) (`GameplayStatics.GetPlayerController` 0)))))

(fn `SetCurrentWeapon`
  (params (NewWeapon :type "/Game/Blueprints/Actors/BP_Weapon Object Reference")))

(fn `SetDamagedHP`
  (params (Damage :type "Float (double-precision)"))
  (set `self.CurrentHP` (- (`self.CurrentHP`) Damage))
  (bind _output_get (set `self.bIsDead` (<= (`self.CurrentHP`) 0.0)))
  (if _output_get
    (`KismetSystemLibrary.PrintString` "꽥" true true (struct :`R` 1.0 :`A` 1.0))
    (`self.DisableInput` (`GameplayStatics.GetPlayerPawn` 0) (`GameplayStatics.GetPlayerController` 0))
    (else
      (`KismetSystemLibrary.PrintString` (`KismetStringLibrary.Concat_StrStr` "CurrentHP : " (`KismetStringLibrary.Conv_DoubleToString` (`self.CurrentHP`))) true true (struct :`R` 1.0 :`A` 1.0)))))

(fn `Swap Weapon1`
  (`/Engine/EditorBlueprintResources/StandardMacros.IsValid` (`self.WeaponSlot1`)
    (:`Is Valid`
      (`/Engine/EditorBlueprintResources/StandardMacros.IsValid` (`self.CurrentWeapon`)
        (:`Is Valid`
          (if (== (`self.CurrentWeapon`) (`self.WeaponSlot1`))
            (set `self.CurrentWeapon` null)
            (`self.K2_AttachToComponent` (`self.WeaponSlot1`) (`self.Mesh`) "WeaponSlot1" "SnapToTarget" "SnapToTarget" "SnapToTarget" true)
            (else
              (set `self.CurrentWeapon` (`self.WeaponSlot1`) :!label _label)
              (`|ExecutionSequence`
                (:`then_0`
                  (`/Engine/EditorBlueprintResources/StandardMacros.IsValid` (`self.WeaponSlot2`)
                    (:`Is Valid`
                      (`self.K2_AttachToComponent` (`self.WeaponSlot2`) (`self.Mesh`) "WeaponSlot2" "SnapToTarget" "SnapToTarget" "SnapToTarget" true))))
                (:`then_1`
                  (`self.K2_AttachToComponent` (`self.WeaponSlot1`) (`self.Mesh`) "R_Weapon" "SnapToTarget" "SnapToTarget" "SnapToTarget" true))))))
        (:`Is Not Valid`
          (goto _label))))))

(fn `Swap Weapon2`
  (`/Engine/EditorBlueprintResources/StandardMacros.IsValid` (`self.WeaponSlot2`)
    (:`Is Valid`
      (`/Engine/EditorBlueprintResources/StandardMacros.IsValid` (`self.CurrentWeapon`)
        (:`Is Valid`
          (if (== (`self.CurrentWeapon`) (`self.WeaponSlot2`))
            (set `self.CurrentWeapon` null)
            (`self.K2_AttachToComponent` (`self.WeaponSlot2`) (`self.Mesh`) "WeaponSlot2" "SnapToTarget" "SnapToTarget" "SnapToTarget" true)
            (else
              (set `self.CurrentWeapon` (`self.WeaponSlot2`) :!label _label)
              (`self.K2_AttachToComponent` (`self.WeaponSlot1`) (`self.Mesh`) "WeaponSlot1" "SnapToTarget" "SnapToTarget" "SnapToTarget" true)
              (`self.K2_AttachToComponent` (`self.WeaponSlot2`) (`self.Mesh`) "R_Weapon" "SnapToTarget" "SnapToTarget" "SnapToTarget" true))))
        (:`Is Not Valid`
          (goto _label))))))

(fn `UserConstructionScript`
  (bind _asbp_game_instance (cast `/Game/Blueprints/Actors/Bear/BP_GameInstance` (`GameplayStatics.GetGameInstance`)))
  (bind _characterdata (`/Game/Blueprints/Actors/Bear/BP_GameInstance.GetCharacterData` _asbp_game_instance (`.Level_6_A1B1A0DB45A1143D48A07B92C6EA64AB` (break `/Game/Blueprints/F_CharacterData` (`self.CurrentCharacterData`)))))
  (bind _output_get (set `self.CurrentCharacterData` _characterdata))
  (set `self.CurrentHP` (`.MaxHP_7_8FF068034D1DE5F5388B87AD55D1D83E` (break `/Game/Blueprints/F_CharacterData` _output_get))))