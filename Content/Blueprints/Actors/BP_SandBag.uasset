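; BP_SandBag is a damageable target pawn that chases the player character and is destroyed when its health runs out.
; PawnSensing sight of a BP_Character triggers an AI MoveTo toward that character.
; AnyDamage prints debug info about the hit, passes damage to SetHealth, which clamps health at zero and flags death, then destroys the actor when dead.
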(event `self.PawnSensing.OnSeePawn`
  (params (Pawn :type "Pawn Object Reference"))
  (bind _asbp_character (cast `/Game/Blueprints/Actors/BP_Character` Pawn))
  (`|AIMoveTo` self (0.0 0.0 0.0) _asbp_character))

(event `self.ReceiveAnyDamage`
  (params (Damage :type "Float (single-precision)") (DamageType :type "DamageType Object Reference") (InstigatedBy :type "Controller Object Reference") (DamageCauser :type "Actor Object Reference"))
  (`KismetSystemLibrary.PrintString` (`KismetStringLibrary.Conv_DoubleToString` Damage))
  (`KismetSystemLibrary.PrintString` (`KismetSystemLibrary.GetDisplayName` InstigatedBy))
  (`KismetSystemLibrary.PrintString` (`KismetSystemLibrary.GetDisplayName` DamageCauser))
  (`self.SetHealth` Damage)
  (if (`self.bIsDead`)
    (`self.K2_DestroyActor`)))

(fn `SetHealth`
  (params (Damage :type "Float (double-precision)"))
  (bind _output_get (set `self.Health` (`KismetMathLibrary.FClamp` (- (`self.Health`) Damage) 0.0 (`self.Health`))))
  (if (== _output_get 0.0)
    (set `self.bIsDead` true)
    (`KismetSystemLibrary.PrintString` "dead")))

(fn `UserConstructionScript`)