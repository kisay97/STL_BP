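; BP_NPC is an AI-controlled NPC character that roams and switches to chasing the first pawn it sees.
; On BeginPlay it writes its roaming range and state to the behavior tree Blackboard and sets walk speed for that state.
; PawnSensing stores the first seen pawn as Enemy, halts movement to interrupt the roaming move task, and sets Chase with a faster speed.
; The Chase state change is not written back to the Blackboard.
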(event `self.ReceiveBeginPlay`
  (bind (_blackboard _keyname) (`self.Get_BB` "NPC_State"))
  (bind (_blackboard_2 _keyname_2) (`self.Get_BB` "RoamingRange"))
  (`BlackboardComponent.SetValueAsFloat` _blackboard_2 _keyname_2 (`self.RoamingRange`))
  (`BlackboardComponent.SetValueAsEnum` _blackboard _keyname (`self.State`))
  (`self.SetWalkSpeedByState` (`self.State`)))

(event `self.PawnSensing.OnSeePawn`
  (params (Pawn :type "Pawn Object Reference"))
  (bind (_blackboard _keyname) (`self.Get_BB` "Enemy"))
  (`self.EnemyPawn`
    (:`then`)
    (:`else`
      (`MovementComponent.StopMovementImmediately` (`self.CharacterMovement`)) ; BTT_NPC_RandomLocation의 Move To Location or Actor를 강제적으로 멈추기 위함
      (bind _output_get (set `self.EnemyPawn` Pawn))
      (`BlackboardComponent.SetValueAsObject` _blackboard _keyname _output_get)
      (bind _output_get_2 (set `self.State` "NewEnumerator2"))
      (`self.SetWalkSpeedByState` _output_get_2))))

(fn `Get_BB`
  (params (value :type Name))
  (returns (blackboard :type "BlackboardComponent Object Reference") (keyName :type Name))
  (return (`AIBlueprintHelperLibrary.GetBlackboard` (`AIBlueprintHelperLibrary.GetAIController` self)) (`KismetSystemLibrary.MakeLiteralName` value)))

(fn `SetWalkSpeedByState`
  (params (Selection :type "/Game/Blueprints/Actors/NPC/E_NPC_State Enum" :default "NewEnumerator0"))
  (bind _charactermovement (`self.CharacterMovement`))
  (switch `/Game/Blueprints/Actors/NPC/E_NPC_State` Selection
    (:`NewEnumerator0`
      (set `CharacterMovementComponent.MaxWalkSpeed` 100.0 _charactermovement))
    (:`NewEnumerator2`
      (set `CharacterMovementComponent.MaxWalkSpeed` 200.0 _charactermovement))))

(fn `UserConstructionScript`)