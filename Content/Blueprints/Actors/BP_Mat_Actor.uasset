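; BP_Mat_Actor is an actor whose Cube changes to a random color when a BP_Character overlaps its Sphere component.
; At BeginPlay it creates a dynamic material instance from the Cube's first material and stores it.
; Each qualifying overlap prints a debug string and sets that instance's Color parameter from random unit vector components, which can be negative, with full alpha.
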(event `self.ReceiveBeginPlay`
  (bind _cube (`self.Cube`))
  (bind _returnvalue (`PrimitiveComponent.CreateDynamicMaterialInstance` _cube 0 (`PrimitiveComponent.GetMaterial` _cube 0) "None"))
  (`PrimitiveComponent.SetMaterial` (`self.Cube`) 0 _returnvalue)
  (set `self.DynamicMaterial` _returnvalue))

(event `self.Sphere.OnComponentBeginOverlap`
  (params (OverlappedComponent :type "PrimitiveComponent Object Reference") (OtherActor :type "Actor Object Reference") (OtherComp :type "PrimitiveComponent Object Reference") (OtherBodyIndex :type Integer) (bFromSweep :type Boolean) (SweepResult :type "HitResult Structure (by ref)"))
  (bind (_returnvalue_x _returnvalue_y _returnvalue_z) (`KismetMathLibrary.BreakVector` (`KismetMathLibrary.RandomUnitVector`)))
  (cast `/Game/Blueprints/Actors/BP_Character` OtherActor)
  (`KismetSystemLibrary.PrintString` "오바랩")
  (`MaterialInstanceDynamic.SetVectorParameterValue` (`self.DynamicMaterial`) "Color" (make `LinearColor` _returnvalue_x _returnvalue_y _returnvalue_z 1.0)))

(fn `UserConstructionScript`)