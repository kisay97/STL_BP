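; BP_Bear is an enemy bear that spots, chases and attacks BP_Character, with health shown on a widget healthbar.
; Sighting the player writes the blackboard target and runs CheckRange, which picks idle/walk, chase or attack by XY distance.
; SetState mirrors the state to the blackboard and sets walk speed.
; SetAttackCollision gathers overlapped actors while enabled, damaging them on disable; incoming damage lowers HP until Death.
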(event `self.PawnSensing.OnSeePawn`
  (params (Pawn :type "Pawn Object Reference"))
  (bind _asbp_character (cast `/Game/Blueprints/Actors/BP_Character` Pawn))
  (set `self.TargetAttackingCharacter` _asbp_character)
  (`BlackboardComponent.SetValueAsObject` (`AIBlueprintHelperLibrary.GetBlackboard` (`self.GetController`)) "TargetPlayer" _asbp_character)
  (`self.CheckRange`))

(event `self.AttackCollision.OnComponentBeginOverlap`
  (params (OverlappedComponent :type "PrimitiveComponent Object Reference") (OtherActor :type "Actor Object Reference") (OtherComp :type "PrimitiveComponent Object Reference") (OtherBodyIndex :type Integer) (bFromSweep :type Boolean) (SweepResult :type "HitResult Structure (by ref)"))
  (`KismetArrayLibrary.Array_AddUnique` (`self.HittedActors`) OtherActor))

(event `self.ReceiveBeginPlay`
  (bind _asumg_enemy_healthbar (cast `/Game/UI/UMG_EnemyHealthbar` (`WidgetComponent.GetWidget` (`self.WB_HPBar`))))
  (set `/Game/UI/UMG_EnemyHealthbar.Onwer` self _asumg_enemy_healthbar))

(event `self.ReceiveAnyDamage`
  (params (Damage :type "Float (single-precision)") (DamageType :type "DamageType Object Reference") (InstigatedBy :type "Controller Object Reference") (DamageCauser :type "Actor Object Reference"))
  (`self.SetHealth` Damage))

(fn `CheckRange`
  (bind _returnvalue (`KismetMathLibrary.VSizeXY` (- (`self.K2_GetActorLocation`) (`self.K2_GetActorLocation` (`self.TargetAttackingCharacter`)))))
  (`/Engine/EditorBlueprintResources/StandardMacros.IsValid` (`self.TargetAttackingCharacter`)
    (:`Is Valid`
      (if (<= _returnvalue (`self.AttackRange`))
        (`self.SetState` "NewEnumerator2")
        (elif (<= _returnvalue (`PawnSensingComponent.SightRadius` (`self.PawnSensing`)))
          (`self.SetState` "NewEnumerator1")
          (else
            (set `self.TargetAttackingCharacter` null)
            (`self.SetState` "NewEnumerator0")))))
    (:`Is Not Valid`
      (`self.SetState` "NewEnumerator0"))))

(fn `GetHPRatio`
  (returns (HPRatio :type "Float (double-precision)"))
  (return (/ (`self.CurrentHP`) (`self.MaxHP`))))

(fn `SetAttackCollision`
  (params (bIsEnable :type Boolean))
  (if bIsEnable
    (`PrimitiveComponent.SetCollisionEnabled` (`self.AttackCollision`) "QueryOnly")
    (else
      (`PrimitiveComponent.SetCollisionEnabled` (`self.AttackCollision`) "NoCollision")
      ;[1 1 1] 맞았던 애들 데미지 주기
      (for _array_element (`self.HittedActors`)
        (`GameplayStatics.ApplyDamage` _array_element (`self.AttackDamage`) (`self.GetController`) self))
      (`KismetArrayLibrary.Array_Clear` (`self.HittedActors`)))))

(fn `SetHealth`
  (params (NewDamage :type "Float (double-precision)"))
  (bind _output_get (set `self.CurrentHP` (- (`self.CurrentHP`) NewDamage)))
  (if (<= _output_get 0.0)
    (`self.SetState` "NewEnumerator3")))

(fn `SetState`
  (params (NewState :type "/Game/Enemy_Bear/E_BearState Enum" :default "NewEnumerator0"))
  (set `self.State` NewState)
  (`BlackboardComponent.SetValueAsEnum` (`AIBlueprintHelperLibrary.GetBlackboard` (`self.GetController`)) "State" (`self.State`))
  (switch `/Game/Enemy_Bear/E_BearState` (`self.State`)
    (:`NewEnumerator0`
      (set `CharacterMovementComponent.MaxWalkSpeed` 200.0 (`self.CharacterMovement`)))
    (:`NewEnumerator1`
      (set `CharacterMovementComponent.MaxWalkSpeed` 400.0 (`self.CharacterMovement`)))
    (:`NewEnumerator2`
      (set `CharacterMovementComponent.MaxWalkSpeed` 0.0 (`self.CharacterMovement`) :!label _label))
    (:`NewEnumerator3`
      (goto _label))))

(fn `UserConstructionScript`
  (`PrimitiveComponent.SetCollisionEnabled` (`self.AttackCollision`) "NoCollision")
  (set `self.CurrentHP` (`self.MaxHP`)))