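; Gate actor that swings open away from the player when the third-person character enters its box trigger.
; CheckDir picks the swing side from a dot product of the gate's forward vector and the player-to-gate direction.
; Open and close timelines lerp SMGate's yaw from its current rotation, each stopping the other first.
; Closing starts on a timer after opening finishes or when the character leaves; OpenGate and CloseGate are uncalled snap-rotation variants.
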(event `self.BoxCollision.OnComponentBeginOverlap`
  (params (OverlappedComponent :type "PrimitiveComponent Object Reference") (OtherActor :type "Actor Object Reference") (OtherComp :type "PrimitiveComponent Object Reference") (OtherBodyIndex :type Integer) (bFromSweep :type Boolean) (SweepResult :type "HitResult Structure (by ref)"))
  (bind (_relativerotation_roll _relativerotation_pitch _relativerotation_yaw) (`KismetMathLibrary.BreakRotator` (`SceneComponent.RelativeRotation` (`self.SM_Gate`))))
  ;[1 1 1] 트리거 조건 예외처리(내 캐릭터인 경우만)
  (if (== (`GameplayStatics.GetObjectClass` OtherActor) (`self.CBP_ThirdPerson_ObjectClassRef`))
    (`self.DoorCloseStop`)
    (`self.CheckDir`)
    (set `self.CurrentYaw` _relativerotation_yaw)
    (set `self.TargetYaw` 90.0)
    (bind (_direction _alpha) (`Timeline|TL_DoorOpen` :!via `PlayFromStart` :!label _label)
      (:`Update`
        (`self.Open_DynamicGate` _alpha))
      (:`Finished`
        (`KismetSystemLibrary.K2_SetTimerDelegate` (delegate `CloseDoorByTimer`) 3.0) ; Time: 유휴시간
      ))))

(event `DoorOpenStop`
  (goto _label :!via `Stop`))

(event `CloseDoorByTimer`
  (bind (_relativerotation_roll _relativerotation_pitch _relativerotation_yaw) (`KismetMathLibrary.BreakRotator` (`SceneComponent.RelativeRotation` (`self.SM_Gate`))))
  (`self.DoorOpenStop` :!label _label_2)
  (set `self.CurrentYaw` _relativerotation_yaw)
  (set `self.TargetYaw` 0.0)
  (bind (_direction _alpha) (`Timeline|TL_DoorClose` :!via `PlayFromStart` :!label _label_3)
    (:`Update`
      (`self.Close_DynamicGate` _alpha))))

(event `self.BoxCollision.OnComponentEndOverlap`
  (params (OverlappedComponent :type "PrimitiveComponent Object Reference") (OtherActor :type "Actor Object Reference") (OtherComp :type "PrimitiveComponent Object Reference") (OtherBodyIndex :type Integer))
  ;[1 1 1] 트리거 조건 예외처리(내 캐릭터인 경우만)
  (if (== (`GameplayStatics.GetObjectClass` OtherActor) (`self.CBP_ThirdPerson_ObjectClassRef`))
    (goto _label_2)))

(event `DoorCloseStop`
  (goto _label_3 :!via `Stop`))

(fn `CheckDir`
  (if (>= (`KismetMathLibrary.Dot_VectorVector` (`KismetMathLibrary.Normal` (- (`self.K2_GetActorLocation`) (`self.K2_GetActorLocation` (`Controller.K2_GetPawn` (`GameplayStatics.GetPlayerController` 0))))) (`self.GetActorForwardVector`)) 0.0)
    (set `self.Dir` 1.0)
    (else
      (set `self.Dir` -1.0))))

(fn `Close_DynamicGate`
  (params (Alpha :type "Float (double-precision)"))
  (`SceneComponent.K2_SetRelativeRotation` (`self.SM_Gate`) (`KismetMathLibrary.MakeRotator` 0.0 0.0 (`KismetMathLibrary.Lerp` (`self.TargetYaw`) (`self.CurrentYaw`) Alpha)) false false))

(fn `CloseGate`
  (params (bIsOpen :type Boolean))
  (locals (Direction :type "Vector Structure"))
  (if bIsOpen
    (bind _output_get (set `local.Direction` (`KismetMathLibrary.Normal` (- (`self.K2_GetActorLocation` (`Controller.K2_GetPawn` (`GameplayStatics.GetPlayerController` 0))) (`self.K2_GetActorLocation`)))))
    (`KismetSystemLibrary.PrintString` (`KismetStringLibrary.Conv_VectorToString` _output_get) true true (struct :`G` 0.66 :`B` 1.0 :`A` 1.0) 20.0)
    (if (>= (.x _output_get) 0.0)
      (`SceneComponent.K2_SetRelativeRotation` :`self` (`self.SM_Gate`))
      (else
        (`SceneComponent.K2_SetRelativeRotation` (`self.SM_Gate`) (struct :`Yaw` 180.0) false false)))
    (else
      (`SceneComponent.K2_SetRelativeRotation` (`self.SM_Gate`) (struct :`Yaw` 90.0) false false))))

(fn `Open_DynamicGate`
  (params (Alpha :type "Float (double-precision)"))
  (`SceneComponent.K2_SetRelativeRotation` (`self.SM_Gate`) (`KismetMathLibrary.MakeRotator` 0.0 0.0 (`KismetMathLibrary.Lerp` (`self.CurrentYaw`) (* (`self.Dir`) (`self.TargetYaw`)) Alpha)) false false))

(fn `OpenGate`
  (params (bIsOpen :type Boolean))
  (locals (Direction :type "Vector Structure"))
  (if bIsOpen
    (bind _output_get (set `local.Direction` (`KismetMathLibrary.Normal` (- (`self.K2_GetActorLocation` (`Controller.K2_GetPawn` (`GameplayStatics.GetPlayerController` 0))) (`self.K2_GetActorLocation`)))))
    (`KismetSystemLibrary.PrintString` (`KismetStringLibrary.Conv_VectorToString` _output_get) true true (struct :`G` 0.66 :`B` 1.0 :`A` 1.0) 20.0)
    (if (>= (.x _output_get) 0.0)
      (`SceneComponent.K2_SetRelativeRotation` :`self` (`self.SM_Gate`))
      (else
        (`SceneComponent.K2_SetRelativeRotation` (`self.SM_Gate`) (struct :`Yaw` 180.0) false false)))
    (else
      (`SceneComponent.K2_SetRelativeRotation` (`self.SM_Gate`) (struct :`Yaw` 90.0) false false))))

(fn `UserConstructionScript`)