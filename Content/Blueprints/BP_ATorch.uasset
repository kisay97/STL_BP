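; BP_ATorch is a torch actor whose PSFire particle effect the player lights with the 1 key.
; Overlap events track whether BP_ThirdPersonCharacter is in range.
; The key calls OnTorch when the character overlaps or the fire is already active, so it never toggles the flame off.
; OnTorch and OffTorch set both fire and overlap flag, though nothing here calls OffTorch.
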(event `self.ReceiveActorBeginOverlap`
  (params (OtherActor :type "Actor Object Reference"))
  (set `self.bOverlap` (== (`GameplayStatics.GetObjectClass` OtherActor) "/Game/ThirdPerson/Blueprints/BP_ThirdPersonCharacter.BP_ThirdPersonCharacter_C")))

(event `self.ReceiveActorEndOverlap`
  (params (OtherActor :type "Actor Object Reference"))
  (if (== (`GameplayStatics.GetObjectClass` OtherActor) "/Game/ThirdPerson/Blueprints/BP_ThirdPersonCharacter.BP_ThirdPersonCharacter_C")
    (set `self.bOverlap` false)))

(event `OffTorch`
  (set `self.bOverlap` false)
  (`ActorComponent.SetActive` (`self.PS_Fire`) false false))

(event `Key|One` :consume false
  (params (Key :type "Key Structure"))
  (:`Pressed`
    (if (or (`ActorComponent.IsActive` (`self.PS_Fire`)) (`self.bOverlap`))
      (`self.OnTorch`))))

(event `OnTorch`
  (set `self.bOverlap` true)
  (`ActorComponent.SetActive` (`self.PS_Fire`) true false))

(fn `UserConstructionScript`)