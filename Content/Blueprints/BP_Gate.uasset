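; Gate actor that swings open away from or toward the player character on overlap and swings shut when the overlap ends.
; An exact class check filters overlaps, then timeline TL_DoorOpen plays or reverses, feeding Alpha to DynamicGate.
; DynamicGate lerps mesh yaw to ±90 degrees, re-checking the player pawn's side on world X every update.
; OpenGate, CloseGate (identical snap-rotation functions) and a front/back check function are never called here.
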(event `self.ReceiveActorBeginOverlap`
  (params (OtherActor :type "Actor Object Reference"))
  ;[1 1 1] 트리거 조건 예외처리(내 캐릭터인 경우만)
  (if (== (`GameplayStatics.GetObjectClass` OtherActor) (`self.CBP_ThirdPerson_ObjectClassRef`))
    (bind (_direction _alpha) (`Timeline|TL_DoorOpen` :!label _label)
      (:`Update`
        (`self.DynamicGate` _alpha)))))

(event `self.ReceiveActorEndOverlap`
  (params (OtherActor :type "Actor Object Reference"))
  ;[1 1 1] 트리거 조건 예외처리(내 캐릭터인 경우만)
  (if (== (`GameplayStatics.GetObjectClass` OtherActor) (`self.CBP_ThirdPerson_ObjectClassRef`))
    (goto _label :!via `Reverse`)))

(event `self.ReceiveTick`
  (params (DeltaSeconds :type "Float (single-precision)")))

(fn `CloseGate`
  (params (bIsOpen :type Boolean))
  (locals (Direction :type "Vector Structure"))
  (if bIsOpen
    (bind _output_get (set `local.Direction` (`KismetMathLibrary.Normal` (- (`self.K2_GetActorLocation` (`Controller.K2_GetPawn` (`GameplayStatics.GetPlayerController` 0))) (`self.K2_GetActorLocation`)))))
    (`KismetSystemLibrary.PrintString` (`KismetStringLibrary.Conv_VectorToString` _output_get) true true (struct :`G` 0.66 :`B` 1.0 :`A` 1.0) 20.0)
    (if (>= (.x _output_get) 0.0)
      (`SceneComponent.K2_SetRelativeRotation` :`self` (`self.StaticMesh`))
      (else
        (`SceneComponent.K2_SetRelativeRotation` (`self.StaticMesh`) (struct :`Yaw` 180.0) false false)))
    (else
      (`SceneComponent.K2_SetRelativeRotation` (`self.StaticMesh`) (struct :`Yaw` 90.0) false false))))

(fn `DynamicGate`
  (params (Alpha :type "Float (double-precision)"))
  (bind _returnvalue_x (`KismetMathLibrary.BreakVector` (`KismetMathLibrary.Normal` (- (`self.K2_GetActorLocation`) (`self.K2_GetActorLocation` (`Controller.K2_GetPawn` (`GameplayStatics.GetPlayerController` 0)))))))
  (if (>= _returnvalue_x 0.0)
    (`SceneComponent.K2_SetRelativeRotation` (`self.StaticMesh`) (`KismetMathLibrary.MakeRotator` 0.0 0.0 (`KismetMathLibrary.Lerp` 0.0 90.0 Alpha)) false false)
    (else
      (`SceneComponent.K2_SetRelativeRotation` (`self.StaticMesh`) (`KismetMathLibrary.MakeRotator` 0.0 0.0 (`KismetMathLibrary.Lerp` 0.0 -90.0 Alpha)) false false))))

(fn `OpenGate`
  (params (bIsOpen :type Boolean))
  (locals (Direction :type "Vector Structure"))
  (if bIsOpen
    (bind _output_get (set `local.Direction` (`KismetMathLibrary.Normal` (- (`self.K2_GetActorLocation` (`Controller.K2_GetPawn` (`GameplayStatics.GetPlayerController` 0))) (`self.K2_GetActorLocation`)))))
    (`KismetSystemLibrary.PrintString` (`KismetStringLibrary.Conv_VectorToString` _output_get) true true (struct :`G` 0.66 :`B` 1.0 :`A` 1.0) 20.0)
    (if (>= (.x _output_get) 0.0)
      (`SceneComponent.K2_SetRelativeRotation` :`self` (`self.StaticMesh`))
      (else
        (`SceneComponent.K2_SetRelativeRotation` (`self.StaticMesh`) (struct :`Yaw` 180.0) false false)))
    (else
      (`SceneComponent.K2_SetRelativeRotation` (`self.StaticMesh`) (struct :`Yaw` 90.0) false false))))

(fn `UserConstructionScript`)

(fn `앞에서들어왔는지_뒤에서들어왔는지_판별함수`
  (returns (isBackEnter :type Boolean))
  (bind _returnvalue_x (`KismetMathLibrary.BreakVector` (`KismetMathLibrary.Normal` (- (`self.K2_GetActorLocation`) (`self.K2_GetActorLocation` (`Controller.K2_GetPawn` (`GameplayStatics.GetPlayerController` 0)))))))
  (if (>= _returnvalue_x 0.0)
    (return false)
    (else
      (return true))))