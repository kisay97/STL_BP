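; Player controller that runs the level-start intro and toggles the in-game menu.
; On BeginPlay it sets game-only input, fades the camera in from black and starts a world-space camera shake after a short delay.
; The Menu input lazily creates and caches UMG_Menu, then adds it to the viewport at high Z-order or removes it.
; Only closing restores game-only input, hides the cursor and unpauses; opening just adds the widget.
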(event `self.ReceiveBeginPlay`
  (`|ExecutionSequence`
    (:`then_0`
      (`WidgetBlueprintLibrary.SetInputMode_GameOnly` self))
    (:`then_1`
      (`PlayerCameraManager.StartCameraFade` :`self` (`self.PlayerCameraManager`) :`FromAlpha` 1.0 :`ToAlpha` 0.0 :`Duration` 2.5)
      (`KismetSystemLibrary.Delay` 1.0)
      (`PlayerCameraManager.StartCameraShake` :`self` (`self.PlayerCameraManager`) :`ShakeClass` "/Game/Blueprints/BP_CameraShake.BP_CameraShake_C" :`Scale` 10.0 :`PlaySpace` "World"))))

(event `InputAction|Menu` :consume false :paused true
  (params (Key :type "Key Structure"))
  (:`Pressed`
    (`self.MenuWidget`
      (:`then`
        (if (`Widget.IsInViewport` (`self.MenuWidget`))
          (`Widget.RemoveFromParent` (`self.MenuWidget`))
          (`WidgetBlueprintLibrary.SetInputMode_GameOnly` (`GameplayStatics.GetPlayerController` 0))
          (set `PlayerController.bShowMouseCursor` false (`GameplayStatics.GetPlayerController` 0))
          (`GameplayStatics.SetGamePaused` false)
          (else
            (`UserWidget.AddToViewport` (stale _output_get) 999 :!label _label))))
      (:`else`
        (bind _returnvalue (`|CreateWidget` "/Game/UI/UMG_Menu.UMG_Menu_C" (`GameplayStatics.GetPlayerController` 0)))
        (bind _output_get (set `self.MenuWidget` _returnvalue))
        (goto _label)))))

(fn `UserConstructionScript`)