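; BP_Character is a player-controlled character Blueprint with basic movement, jumping, camera look and zoom.
; Move axes feed AddMovementInput along forward and right vectors built only from control rotation yaw, keeping movement camera-relative and level.
; Turn and look axes drive controller yaw and pitch, while the mouse wheel changes spring arm length without clamping.
; Jump press and release call Jump and StopJumping; OnJumped and the construction script are empty.
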(event `InputAction|Jump`
  (params (Key :type "Key Structure"))
  (:`Pressed`
    (`self.Jump`))
  (:`Released`
    (`self.StopJumping`) ; 살짝 점프, 긴 점프 같은 것을 처리할 수 있음.\n기본적으로 그런 기능을 넣지 않더라도 Stop Jumping은 Jump 입력 액션 Released에 넣어준다고 함.
  ))

(event `self.OnJumped`)

(event `InputAxisKey|MouseWheelAxis`
  (params (AxisValue :type "Float (single-precision)"))
  (bind _springarm (`self.SpringArm`))
  (set `SpringArmComponent.TargetArmLength` (+ (* AxisValue -10.0) (`SpringArmComponent.TargetArmLength` _springarm)) _springarm))

(event `InputAxis|MoveForward / MoveBackward`
  (params (AxisValue :type "Float (single-precision)"))
  (bind (_returnvalue_roll _returnvalue_pitch _returnvalue_yaw) (`KismetMathLibrary.BreakRotator` (`self.GetControlRotation`)))
  (`self.AddMovementInput` (`KismetMathLibrary.GetForwardVector` (`KismetMathLibrary.MakeRotator` 0.0 0.0 _returnvalue_yaw)) AxisValue) ; 속도는 캐릭터가 들고있다.(가속도, 최대속도 등)\n조작계에 따른 내 캐릭터의 정방을 World Direction으로 줘야한다.
)

(event `InputAxis|MoveRight / MoveLeft`
  (params (AxisValue :type "Float (single-precision)"))
  (bind (_returnvalue_roll _returnvalue_pitch _returnvalue_yaw) (`KismetMathLibrary.BreakRotator` (`self.GetControlRotation`)))
  (`self.AddMovementInput` (`KismetMathLibrary.GetRightVector` (`KismetMathLibrary.MakeRotator` 0.0 0.0 _returnvalue_yaw)) AxisValue) ; 속도는 캐릭터가 들고있다.(가속도, 최대속도 등)
)

(event `InputAxis|TurnRight / Left`
  (params (AxisValue :type "Float (single-precision)"))
  (`self.AddControllerYawInput` AxisValue))

(event `InputAxis|LookUp / Down`
  (params (AxisValue :type "Float (single-precision)"))
  (`self.AddControllerPitchInput` AxisValue))

(fn `UserConstructionScript`)